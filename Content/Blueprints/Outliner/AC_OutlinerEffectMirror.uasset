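; Actor component that changes the outline on its owner's static mesh, apparently for mirrors, when the player character is nearby.
; On BeginPlay it finds the owner's StaticMesh and Sphere components and builds a dynamic M_Outline material with configurable color and thickness.
; Sphere overlap by the player sets that material as the mesh's overlay.
; Leaving restores the fixed MI_OutlineMiroirs overlay rather than clearing it.
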(event `self.ReceiveBeginPlay`
  (bind _returnvalue (`self.GetOwner`))
  ; Recupere le static mesh
  (set `self.TargetMesh` (`Actor.GetComponentByClass` _returnvalue "/Script/Engine.StaticMeshComponent"))
  (set `self.Sphere` (`Actor.GetComponentByClass` _returnvalue "/Script/Engine.SphereComponent"))
  (`|ExecutionSequence`
    (:`then_0`
      ; Crée le matériau et applique les preferences choisies
      (bind _returnvalue_2 (`KismetMaterialLibrary.CreateDynamicMaterialInstance` "/Game/Blueprints/Outliner/M_Outline.M_Outline" "MI_Outline"))
      (bind _output_get (set `self.DynamicMaterial` _returnvalue_2))
      (`MaterialInstanceDynamic.SetVectorParameterValue` _output_get "Color" (`self.OutlineColor`))
      (`MaterialInstanceDynamic.SetScalarParameterValue` _output_get "LineThickness" (`self.OutlineThickness`)))
    (:`then_1`
      (bind _sphere (`self.Sphere`)
        (:`then`
          (add `PrimitiveComponent.OnComponentBeginOverlap` _sphere (delegate `BeginOverlap`)))
        (:`else`)))
    (:`then_2`
      (bind _sphere_2 (`self.Sphere`)
        (:`then`
          (add `PrimitiveComponent.OnComponentEndOverlap` _sphere_2 (delegate `EndOverlap`)))
        (:`else`)))))

(event `BeginOverlap`
  (params (OverlappedComponent :type "PrimitiveComponent Object Reference") (OtherActor :type "Actor Object Reference") (OtherComp :type "PrimitiveComponent Object Reference") (OtherBodyIndex :type Integer) (bFromSweep :type Boolean) (SweepResult :type "HitResult Structure (by ref)"))
  ; Gestion des overlaps (ajout du overlay material)
  (if (== OtherActor (`GameplayStatics.GetPlayerCharacter` 0))
    (`MeshComponent.SetOverlayMaterial` (`self.TargetMesh`) (`self.DynamicMaterial`))))

(event `EndOverlap`
  (params (OverlappedComponent :type "PrimitiveComponent Object Reference") (OtherActor :type "Actor Object Reference") (OtherComp :type "PrimitiveComponent Object Reference") (OtherBodyIndex :type Integer))
  ; Gestion des overlaps (ajout du overlay material)
  (if (== OtherActor (`GameplayStatics.GetPlayerCharacter` 0))
    (`MeshComponent.SetOverlayMaterial` (`self.TargetMesh`) "/Game/Blueprints/Outliner/MI_OutlineMiroirs.MI_OutlineMiroirs")))