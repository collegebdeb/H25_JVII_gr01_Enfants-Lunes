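; Actor component that outlines its owner's static mesh while an actor overlaps an assigned TriggerSphere.
; On BeginPlay it finds the owner's StaticMeshComponent and creates a dynamic M_Outline instance with the configured color and thickness.
; If TriggerSphere is valid, its overlap events set that instance as the mesh's overlay material and clear it on exit, without filtering the overlapping actor.
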(event `self.ReceiveBeginPlay`
  ; Recupere le static mesh
  (set `self.TargetMesh` (`Actor.GetComponentByClass` (`self.GetOwner`) "/Script/Engine.StaticMeshComponent"))
  (`|ExecutionSequence`
    (:`then_0`
      (bind _returnvalue (`KismetMaterialLibrary.CreateDynamicMaterialInstance` "/Game/Blueprints/Outliner/M_Outline.M_Outline" "MI_Outline"))
      (bind _output_get (set `self.DynamicMaterial` _returnvalue))
      (`MaterialInstanceDynamic.SetVectorParameterValue` _output_get "Color" (`self.OutlineColor`))
      (`MaterialInstanceDynamic.SetScalarParameterValue` _output_get "LineThickness" (`self.OutlineThickness`)))
    (:`then_1`
      ; Gestion des overlaps (ajout du overlay material)
      (bind _triggersphere (`self.TriggerSphere`)
        (:`then`
          (add `Actor.OnActorBeginOverlap` _triggersphere (delegate `HandleBeginOverlap`))
          (add `Actor.OnActorEndOverlap` _triggersphere (delegate `HandleEndOverlap`)))
        (:`else`)))))

(event `HandleEndOverlap`
  (params (OverlappedActor :type "Actor Object Reference") (OtherActor :type "Actor Object Reference"))
  ; Gestion des overlaps (ajout du overlay material)
  (`MeshComponent.SetOverlayMaterial` (`self.TargetMesh`) null))

(event `HandleBeginOverlap`
  (params (OverlappedActor :type "Actor Object Reference") (OtherActor :type "Actor Object Reference"))
  ; Gestion des overlaps (ajout du overlay material)
  (`MeshComponent.SetOverlayMaterial` (`self.TargetMesh`) (`self.DynamicMaterial`)))