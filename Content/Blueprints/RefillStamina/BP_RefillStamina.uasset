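; BP_RefillStamina is a zone that refills the StaminaLight of the player's BP_Leila character while she overlaps its Box.
; Entering starts her regen loop and plays the refill sound, or fades in the end sound if StaminaLight is already full.
; Leaving stops the loop and fades out both 2D sounds, which are created on BeginPlay.
; Fullness is checked only on entry, so filling up inside the box does not switch sounds.
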(event `self.ReceiveBeginPlay`
  (bind _asbp_leila (cast `/Game/Blueprints/BP_Leila` (`GameplayStatics.GetPlayerCharacter` 0)))
  (set `self.As BP Leila` _asbp_leila)
  (bind _returnvalue (`GameplayStatics.CreateSound2D` "/Game/Sons/Stamina/S_Refill.S_Refill" 1.0 1.0 0.0 null))
  (set `self.RefillSound` _returnvalue)
  (bind _returnvalue_2 (`GameplayStatics.CreateSound2D` "/Game/Sons/Stamina/S_RefillEnd.S_RefillEnd" 1.0 1.0 0.0 null))
  (set `self.EndRefillSound` _returnvalue_2))

(event `self.Box.OnComponentBeginOverlap`
  (params (OverlappedComponent :type "PrimitiveComponent Object Reference") (OtherActor :type "Actor Object Reference") (OtherComp :type "PrimitiveComponent Object Reference") (OtherBodyIndex :type Integer) (bFromSweep :type Boolean) (SweepResult :type "HitResult Structure (by ref)"))
  (if (== OtherActor (`self.As BP Leila`))
    (`/Game/Blueprints/BP_Leila.StartSaminaRegenLoop` (`self.As BP Leila`))
    (if (== (`/Game/Blueprints/BP_Leila.StaminaLight` (`self.As BP Leila`)) 100.0)
      (bind _refillsound (`self.RefillSound`)
        (:`then`
          (if (`AudioComponent.IsPlaying` _refillsound)
            (bind _refillsound_2 (`self.RefillSound`)
              (:`then`
                (`AudioComponent.FadeOut` _refillsound_2 0.3 0.0 "Linear"))
              (:`else`))))
        (:`else`
          _))
      (bind _endrefillsound (`self.EndRefillSound`)
        (:`then`
          (`AudioComponent.FadeIn` _endrefillsound 0.3 1.0 0.0 "Linear"))
        (:`else`
          (bind _returnvalue (`GameplayStatics.CreateSound2D` "/Game/Sons/Stamina/S_RefillEnd.S_RefillEnd" 1.0 1.0 0.0 null))
          (bind _output_get (set `self.EndRefillSound` _returnvalue))
          (`AudioComponent.FadeIn` _output_get 0.5 1.0 0.0 "Linear")))
      (else
        (bind _refillsound_3 (`self.RefillSound`)
          (:`then`
            (`AudioComponent.Play` _refillsound_3 0.0))
          (:`else`
            (bind _returnvalue_2 (`GameplayStatics.CreateSound2D` "/Game/Sons/Stamina/S_Refill.S_Refill" 1.0 1.0 0.0 null))
            (bind _output_get_2 (set `self.RefillSound` _returnvalue_2))
            (`AudioComponent.Play` _output_get_2 0.0)))))))

(event `self.Box.OnComponentEndOverlap`
  (params (OverlappedComponent :type "PrimitiveComponent Object Reference") (OtherActor :type "Actor Object Reference") (OtherComp :type "PrimitiveComponent Object Reference") (OtherBodyIndex :type Integer))
  (if (== OtherActor (`self.As BP Leila`))
    (`/Game/Blueprints/BP_Leila.StopStaminaRegenLoop` (`self.As BP Leila`))
    (`|ExecutionSequence`
      (:`then_0`
        (bind _refillsound (`self.RefillSound`)
          (:`then`
            (if (`AudioComponent.IsPlaying` _refillsound)
              (`AudioComponent.FadeOut` _refillsound 0.5 0.0 "Linear")))
          (:`else`)))
      (:`then_1`
        (bind _endrefillsound (`self.EndRefillSound`)
          (:`then`
            (if (`AudioComponent.IsPlaying` _endrefillsound)
              (`AudioComponent.FadeOut` _endrefillsound 0.5 0.0 "Linear")))
          (:`else`))))))

(fn `UserConstructionScript`)