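; Interaction prompt for the second gear (engrenage) puzzle element, showing an E-key icon when Leila is in range.
; Box overlap reveals the widget only if Leila's CanActivateEngrenage2 is set and she holds no object; any end overlap hides it.
; Tick also hides it while she is grabbing, using the player reference cached at BeginPlay.
; HidePromptEngrenage2 lets the prompt be hidden once the puzzle is solved.
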(event `self.ReceiveBeginPlay`
  (bind _asbp_leila (cast `/Game/Blueprints/BP_Leila` (`GameplayStatics.GetPlayerCharacter` 0)))
  (bind _output_get (set `self.As BP Leila` _asbp_leila))
  (`self.EnableInput` _output_get (`GameplayStatics.GetPlayerController` 0))
  (`SceneComponent.SetVisibility` (`self.Widget`) false false))

(event `self.Box.OnComponentBeginOverlap`
  (params (OverlappedComponent :type "PrimitiveComponent Object Reference") (OtherActor :type "Actor Object Reference") (OtherComp :type "PrimitiveComponent Object Reference") (OtherBodyIndex :type Integer) (bFromSweep :type Boolean) (SweepResult :type "HitResult Structure (by ref)"))
  ; Trigger Box qui active et désactive l'icône E quand le joueur passe dessus
  (bind _asbp_leila (cast `/Game/Blueprints/BP_Leila` OtherActor))
  (if (`/Game/Blueprints/BP_Leila.CanActivateEngrenage2` _asbp_leila)
    (`self.DisplaysE`)))

(event `self.Box.OnComponentEndOverlap`
  (params (OverlappedComponent :type "PrimitiveComponent Object Reference") (OtherActor :type "Actor Object Reference") (OtherComp :type "PrimitiveComponent Object Reference") (OtherBodyIndex :type Integer))
  ; Trigger Box qui active et désactive l'icône E quand le joueur passe dessus
  (`self.ClosesDisplayE`))

(event `HidePromptEngrenage2`
  ; Option de cacher l'icône E quand l'énigme est déjà résolue
  (`SceneComponent.SetVisibility` (`self.Widget`) false false))

(event `DisplaysE`
  (`/Engine/EditorBlueprintResources/StandardMacros.IsValid` (`self.Widget`)
    (:`Is Valid`
      (bind _as_bp_leila (`self.As BP Leila`)
        (:`then`
          (if (not (`/Game/Blueprints/BP_Leila.GrabbingObject` _as_bp_leila))
            (`SceneComponent.SetVisibility` (`self.Widget`) true false)))
        (:`else`)))))

(event `ClosesDisplayE`
  (`/Engine/EditorBlueprintResources/StandardMacros.IsValid` (`self.Widget`)
    (:`Is Valid`
      (`SceneComponent.SetVisibility` (`self.Widget`) false false))))

(event `self.ReceiveTick`
  (params (DeltaSeconds :type "Float (single-precision)"))
  (if (`/Game/Blueprints/BP_Leila.GrabbingObject` (`self.As BP Leila`))
    (`self.ClosesDisplayE`)))

(fn `UserConstructionScript`)