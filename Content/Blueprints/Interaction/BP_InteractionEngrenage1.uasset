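; BP_InteractionEngrenage1 is an interaction trigger that shows an "E" key prompt for the first gear (engrenage) puzzle.
; A trigger box shows and hides the prompt widget as it is entered and left, without filtering the overlapping actor.
; IA_Interaction hides the prompt while held inside the box and restores it on release.
; HidePromptEngrenage1 permanently disables the prompt, intended for when the puzzle is solved.
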(event `self.ReceiveBeginPlay`
  (`self.EnableInput` (`GameplayStatics.GetPlayerController` 0)))

(event `self.Box.OnComponentBeginOverlap`
  (params (OverlappedComponent :type "PrimitiveComponent Object Reference") (OtherActor :type "Actor Object Reference") (OtherComp :type "PrimitiveComponent Object Reference") (OtherBodyIndex :type Integer) (bFromSweep :type Boolean) (SweepResult :type "HitResult Structure (by ref)"))
  ; Trigger Box qui active et désactive l'icône E quand le joueur passe dessus
  (set `self.InTriggerBox` true)
  (if (`self.PromptEnabled`)
    (if (not (`self.KeyEPressed`))
      (`SceneComponent.SetVisibility` (`self.Widget`) true false))))

(event `self.Box.OnComponentEndOverlap`
  (params (OverlappedComponent :type "PrimitiveComponent Object Reference") (OtherActor :type "Actor Object Reference") (OtherComp :type "PrimitiveComponent Object Reference") (OtherBodyIndex :type Integer))
  ; Trigger Box qui active et désactive l'icône E quand le joueur passe dessus
  (set `self.InTriggerBox` false)
  (`SceneComponent.SetVisibility` (`self.Widget`) false false))

(event `HidePromptEngrenage1`
  ; Option de cacher l'icône E quand l'énigme est déjà résolue
  (set `self.PromptEnabled` false)
  (`SceneComponent.SetVisibility` (`self.Widget`) false false))

(event `EnhancedInput|/Game/Blueprints/InputActions/IA_Interaction`
  (params (ActionValue :type Boolean) (ElapsedSeconds :type "Float (double-precision)") (TriggeredSeconds :type "Float (double-precision)") (InputAction :type "InputAction Object Reference" :default "/Game/Blueprints/InputActions/IA_Interaction.IA_Interaction"))
  ; Quand le joueur clique sur E, le prompt disparaît, et quand le joueur relâche la touche E, le prompt réapparaît
  (:`Started`
    (set `self.KeyEPressed` true)
    (if (`self.PromptEnabled`)
      (if (`self.InTriggerBox`)
        (`SceneComponent.SetVisibility` (`self.Widget`) false false)
        (`KismetSystemLibrary.PrintString` "E Pressed"))))
  (:`Completed`
    (set `self.KeyEPressed` false)
    (if (`self.PromptEnabled`)
      (if (`self.InTriggerBox`)
        (`SceneComponent.SetVisibility` (`self.Widget`) true false)
        (`KismetSystemLibrary.PrintString` "E Unpressed")))))

(fn `UserConstructionScript`)