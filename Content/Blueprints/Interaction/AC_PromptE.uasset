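; AC_PromptE is an actor component that shows an "E" interaction prompt when something overlaps its owner's trigger sphere.
; On BeginPlay it finds the owner's sphere and widget components, hides the widget, binds the overlap events and caches the player as BP_Leila.
; Overlap start shows the widget unless Leila is grabbing an object, without filtering the overlapping actor.
; Overlap end hides it, as does Tick whenever she is grabbing.
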(event `OnComponentBeginOverlap_Event`
  (params (OverlappedComponent :type "PrimitiveComponent Object Reference") (OtherActor :type "Actor Object Reference") (OtherComp :type "PrimitiveComponent Object Reference") (OtherBodyIndex :type Integer) (bFromSweep :type Boolean) (SweepResult :type "HitResult Structure (by ref)"))
  ; trigger Box qui activer et désactive l'icône E quand le joueur passe dessus
  (`self.DisplaysE`))

(event `OnComponentEndOverlap_Event`
  (params (OverlappedComponent :type "PrimitiveComponent Object Reference") (OtherActor :type "Actor Object Reference") (OtherComp :type "PrimitiveComponent Object Reference") (OtherBodyIndex :type Integer))
  ; trigger Box qui activer et désactive l'icône E quand le joueur passe dessus
  (`self.ClosesDisplayE`))

(event `self.ReceiveBeginPlay`
  (bind _returnvalue (`self.GetOwner`))
  (`|ExecutionSequence`
    (:`then_0`
      (set `self.Sphere` (`Actor.GetComponentByClass` _returnvalue "/Script/Engine.SphereComponent"))
      (bind _output_get (set `self.Widget` (`Actor.GetComponentByClass` _returnvalue "/Script/UMG.WidgetComponent")))
      (`SceneComponent.SetVisibility` _output_get false false)
      (bind _sphere (`self.Sphere`)
        (:`then`
          (add `PrimitiveComponent.OnComponentBeginOverlap` _sphere (delegate `OnComponentBeginOverlap_Event`))
          (add `PrimitiveComponent.OnComponentEndOverlap` _sphere (delegate `OnComponentEndOverlap_Event`)))
        (:`else`)))
    (:`then_1`
      (bind _asbp_leila (cast `/Game/Blueprints/BP_Leila` (`GameplayStatics.GetPlayerCharacter` 0)))
      (set `self.As BP Leila` _asbp_leila))))

(event `DisplaysE`
  (`/Engine/EditorBlueprintResources/StandardMacros.IsValid` (`self.Widget`)
    (:`Is Valid`
      (bind _as_bp_leila (`self.As BP Leila`)
        (:`then`
          (if (not (`/Game/Blueprints/BP_Leila.GrabbingObject` _as_bp_leila))
            (`SceneComponent.SetVisibility` (`self.Widget`) true false)))
        (:`else`)))))

(event `ClosesDisplayE`
  (`/Engine/EditorBlueprintResources/StandardMacros.IsValid` (`self.Widget`)
    (:`Is Valid`
      (`SceneComponent.SetVisibility` (`self.Widget`) false false))))

(event `self.ReceiveTick`
  (params (DeltaSeconds :type "Float (single-precision)"))
  (if (`/Game/Blueprints/BP_Leila.GrabbingObject` (`self.As BP Leila`))
    (`self.ClosesDisplayE`)))