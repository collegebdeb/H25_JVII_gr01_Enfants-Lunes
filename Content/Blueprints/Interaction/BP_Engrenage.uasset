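; BP_Engrenage is a gear actor that shows an "E" interaction prompt when something approaches it.
; Box overlap shows WidgetE if CanShowPrompt is set and hides it on exit, without filtering the overlapping actor.
; IA_Interaction handlers, marked as a non-working test, hide the prompt on Triggered and show it on Canceled regardless of overlap or CanShowPrompt.
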(event `self.Box.OnComponentBeginOverlap`
  (params (OverlappedComponent :type "PrimitiveComponent Object Reference") (OtherActor :type "Actor Object Reference") (OtherComp :type "PrimitiveComponent Object Reference") (OtherBodyIndex :type Integer) (bFromSweep :type Boolean) (SweepResult :type "HitResult Structure (by ref)"))
  ; Prompt E apparâit quand on s'approche de l'engrenage
  (if (`self.CanShowPrompt`)
    (`SceneComponent.SetVisibility` (`self.Widget E`) true false)))

(event `self.Box.OnComponentEndOverlap`
  (params (OverlappedComponent :type "PrimitiveComponent Object Reference") (OtherActor :type "Actor Object Reference") (OtherComp :type "PrimitiveComponent Object Reference") (OtherBodyIndex :type Integer))
  ; Prompt E apparâit quand on s'approche de l'engrenage
  (`SceneComponent.SetVisibility` (`self.Widget E`) false false))

(event `EnhancedInput|/Game/Blueprints/InputActions/IA_Interaction`
  (params (ActionValue :type Boolean) (ElapsedSeconds :type "Float (double-precision)") (TriggeredSeconds :type "Float (double-precision)") (InputAction :type "InputAction Object Reference" :default "/Game/Blueprints/InputActions/IA_Interaction.IA_Interaction"))
  ; Test (fonctionne pas)
  (:`Triggered`
    (`SceneComponent.SetVisibility` (`self.Widget E`) false false))
  (:`Canceled`
    (`SceneComponent.SetVisibility` (`self.Widget E`) true false)))

(fn `UserConstructionScript`)