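; Interaction actor for a padlock puzzle that controls an "E" key prompt widget around a trigger box.
; Box overlaps show and hide the widget for any actor, and HidePrompt hides it for a solved puzzle.
; Tick sets the widget visible every frame, overriding both hides.
; BeginPlay caches the BP_Leila player, but the player-filtered overlap and ActivationLock logic is disconnected and never runs.
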(event `self.ReceiveBeginPlay`
  (bind _asbp_leila (cast `/Game/Blueprints/BP_Leila` (`GameplayStatics.GetPlayerCharacter` 0)))
  (set `self.As BP Leila` _asbp_leila))

(event `self.Box.OnComponentBeginOverlap`
  (params (OverlappedComponent :type "PrimitiveComponent Object Reference") (OtherActor :type "Actor Object Reference") (OtherComp :type "PrimitiveComponent Object Reference") (OtherBodyIndex :type Integer) (bFromSweep :type Boolean) (SweepResult :type "HitResult Structure (by ref)"))
  ; trigger Box qui activer et désactive l'icône E quand le joueur passe dessus
  (`SceneComponent.SetVisibility` (`self.Widget`) true false))

(event `self.Box.OnComponentEndOverlap`
  (params (OverlappedComponent :type "PrimitiveComponent Object Reference") (OtherActor :type "Actor Object Reference") (OtherComp :type "PrimitiveComponent Object Reference") (OtherBodyIndex :type Integer))
  ; trigger Box qui activer et désactive l'icône E quand le joueur passe dessus
  (`SceneComponent.SetVisibility` (`self.Widget`) false false))

(event `HidePrompt`
  ; Option de cacher l'icône E quand l'énigme est déjà résolue
  (`SceneComponent.SetVisibility` (`self.Widget`) false false))

(event `self.ReceiveTick`
  (params (DeltaSeconds :type "Float (single-precision)"))
  (`SceneComponent.SetVisibility` (`self.Widget`) true false))

(fn `UserConstructionScript`)