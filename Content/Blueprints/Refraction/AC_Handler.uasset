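; Actor component for laser refraction puzzles that relays laser hit and forced activation events to the owner's other BPI_Lasers components.
; BeginPlay gathers those components, sets the meshes' laser trace response and, if inverted, sends stop-hit to emitters.
; Start and stop events track lasers and, unless locked, fire immediately or via a reversible looping timer that broadcasts progress.
; Forced activation requires all linked external components active, and replays lasers when AC_Bounce exists.
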(event `self.ReceiveBeginPlay`
  (`|ExecutionSequence`
    (:`then_0`
      (bind _output_get (set `self.LinkedComponents` (`Actor.GetComponentsByInterface` (`self.GetOwner`) "/Game/Blueprints/Refraction/BPI_Lasers.BPI_Lasers_C")))
      (`KismetArrayLibrary.Array_RemoveItem` _output_get self)
      (for _array_element (`Actor.K2_GetComponentsByClass` (`self.GetOwner`) "/Script/Engine.StaticMeshComponent")
        (`PrimitiveComponent.SetCollisionResponseToChannel` _array_element "ECC_GameTraceChannel1" (select `bool` (`self.IsBlocking?`) :`false` "ECR_Overlap" :`true` "ECR_Block" :!type "ECollisionResponse Enum"))))
    (:`then_1`
      (if (`self.InvertSystem?`)
        (for _array_element_2 (`Actor.K2_GetComponentsByClass` (`self.GetOwner`) "/Game/Blueprints/Refraction/SC_Emitter.SC_Emitter_C")
          (`/Game/Blueprints/Refraction/SC_Emitter.LaserStopHitting` _array_element_2 null))))))

(event `CE_TimerFinishedActivate`
  (bind _array_element (`self.ForEachComponents` :!label _label)
    (:`LoopBody`
      (message `/Game/Blueprints/Refraction/BPI_Lasers.LaserStartHitting` _array_element (stale `/Game/Blueprints/Refraction/BPI_Lasers.LaserStartHitting` Input) (stale `/Game/Blueprints/Refraction/BPI_Lasers.LaserStartHitting` `Hit Info`)))
    (:`Completed`
      (`self.ActivateHandler` self))))

(event `/Game/Blueprints/Refraction/BPI_Lasers.LaserStartHitting`
  (params (Input :type "/Game/Blueprints/Refraction/A_Laser Object Reference") (`Hit Info` :type "HitResult Structure"))
  (`self.Laser Added` Input)
  (`self.IsNotLocked`
    (:`Not Locked`
      (if (not (`self.UseTimer`))
        (goto _label)
        (else
          (set `self.ReverseTimer` false)
          (`self.StartTimer` false))))))

(event `CE_TimerFinishedDeactivate`
  (bind (_array_element _laser) (`self.ForEachLaser` :!label _label_2)
    (:`LoopBody`
      (message `/Game/Blueprints/Refraction/BPI_Lasers.LaserStopHitting` _array_element _laser))
    (:`Completed Loop`
      (bind _array_element_2 (`self.ForEachComponents`)
        (:`LoopBody`
          (message `/Game/Blueprints/Refraction/BPI_Lasers.LaserStopHitting` _array_element_2 (stale `/Game/Blueprints/Refraction/BPI_Lasers.LaserStopHitting` Input)))
        (:`Completed`
          (`self.DeactivateHandler` self))))))

(event `/Game/Blueprints/Refraction/BPI_Lasers.LaserStopHitting`
  (params (Input :type "/Game/Blueprints/Refraction/A_Laser Object Reference"))
  (`self.Laser Removed` Input)
  (`self.IsNotLocked`
    (:`Not Locked`
      (if (not (`self.UseTimer`))
        (goto _label_2)
        (else
          (set `self.ReverseTimer` true)
          (`self.StartTimer` false))))))

(event `/Game/Blueprints/Refraction/BPI_Lasers.LaserUpdateHitting`
  (params (Input :type "/Game/Blueprints/Refraction/A_Laser Object Reference") (`Hit Info` :type "HitResult Structure"))
  (bind _array_element (`self.ForEachComponents`)
    (:`LoopBody`
      (message `/Game/Blueprints/Refraction/BPI_Lasers.LaserUpdateHitting` _array_element Input `Hit Info`))))

(event `CE_Ext_TimerActivate`
  (bind _array_element (`self.ForEachComponents` :!label _label_3)
    (:`LoopBody`
      (message `/Game/Blueprints/Refraction/BPI_Lasers.ForceActivation` _array_element (stale `/Game/Blueprints/Refraction/BPI_Lasers.ForceActivation` ApplyConditions)))
    (:`Completed`
      (`/Engine/EditorBlueprintResources/StandardMacros.IsValid` (`Actor.GetComponentByClass` (`self.GetOwner`) "/Game/Blueprints/Refraction/AC_Bounce.AC_Bounce_C")
        (:`Is Valid`
          (bind (_array_element_2 _laser _hit_result) (`self.ForEachLaser`)
            (:`LoopBody`
              (message `/Game/Blueprints/Refraction/BPI_Lasers.LaserStartHitting` _array_element_2 _laser _hit_result))
            (:`Completed Loop`
              (`self.ActivateHandler` self))))))))

(event `/Game/Blueprints/Refraction/BPI_Lasers.ForceActivation`
  (params (ApplyConditions :type Boolean))
  (if (`self.AreAllCompsActivated?`)
    (if (not (`self.UseTimer`))
      (goto _label_3)
      (else
        (set `self.ReverseTimer` false)
        (`self.StartTimer` true)))))

(event `CE_Ext_TimerDeactivate`
  (bind _array_element (`self.ForEachComponents` :!label _label_4)
    (:`LoopBody`
      (message `/Game/Blueprints/Refraction/BPI_Lasers.ForceDeactivation` _array_element (stale `/Game/Blueprints/Refraction/BPI_Lasers.ForceDeactivation` ApplyConditions)))
    (:`Completed`
      (`/Engine/EditorBlueprintResources/StandardMacros.IsValid` (`Actor.GetComponentByClass` (`self.GetOwner`) "/Game/Blueprints/Refraction/AC_Bounce.AC_Bounce_C")
        (:`Is Valid`
          (bind (_array_element_2 _laser) (`self.ForEachLaser`)
            (:`LoopBody`
              (message `/Game/Blueprints/Refraction/BPI_Lasers.LaserStopHitting` _array_element_2 _laser))
            (:`Completed Loop`
              (`self.DeactivateHandler` self))))))))

(event `/Game/Blueprints/Refraction/BPI_Lasers.ForceDeactivation`
  (params (ApplyConditions :type Boolean))
  (if (not (`self.UseTimer`))
    (goto _label_4)
    (else
      (set `self.ReverseTimer` true)
      (`self.StartTimer` true))))

(fn `AreAllCompsActivated?`
  (returns (ReturnValue :type Boolean))
  (for _array_element (`self.LinkedExternalComps`)
    (if (not (`/Game/Blueprints/Refraction/AC_External.IsCompActivated?` _array_element))
      (return false)))
  (return true))

(fn `CanActivate?`
  (returns (`Succes?` :type Boolean))
  (locals (`L-FilteredLasers` :type "Array of /Game/Blueprints/Refraction/A_Laser Object Reference"))
  (bind _output_get (set `local.L-FilteredLasers` (`self.FilteredLasers`)))
  (if (and (`KismetArrayLibrary.Array_IsEmpty` _output_get) (`self.IsLinked`))
    (return false)
    (elif (`KismetArrayLibrary.Array_IsEmpty` (`self.LaserRules`))
      (if (`self.IsLinked`)
        (return (`self.AreAllCompsActivated?`))
        (else
          (return true)))
      (elif (> (`KismetArrayLibrary.Array_Length` (`self.LaserRules`)) (`KismetArrayLibrary.Array_Length` (`local.L-FilteredLasers`)))
        (return false)
        (else
          (return true))))))

(fn `ExternalUpdateTimer`
  (if (select `bool` (`self.ReverseTimer`) :`false` (>= (`self.TimerAlpha`) 1.0) :`true` (<= (`self.TimerAlpha`) 0.0))
    (`KismetSystemLibrary.K2_ClearAndInvalidateTimerHandle` (`self.TimerHandle`))
    (if (`self.ReverseTimer`)
      (`self.CE_Ext_TimerDeactivate`)
      (else
        (`self.CE_Ext_TimerActivate`)))
    (else
      (set `self.TimerAlpha` (+ (* (* (/ 1.0 (`self.Duration`)) (`self.Substep`)) (`KismetMathLibrary.SelectFloat` -1.0 1.0 (`self.ReverseTimer`))) (`self.TimerAlpha`)))
      (`self.UpdateHandler` (`self.TimerAlpha`)))))

(fn `Laser Added`
  (params (NewItem :type "/Game/Blueprints/Refraction/A_Laser Object Reference (by ref)"))
  (`KismetArrayLibrary.Array_AddUnique` (`self.LasersInQueue`) NewItem))

(fn `Laser Removed`
  (params (NewItem :type "/Game/Blueprints/Refraction/A_Laser Object Reference (by ref)"))
  (`KismetArrayLibrary.Array_RemoveItem` (`self.LasersInQueue`)))

(fn `StartTimer`
  (params (ExternalTimer :type Boolean))
  (if (`KismetSystemLibrary.K2_TimerExistsHandle` (`self.TimerHandle`))
    (`KismetSystemLibrary.K2_ClearAndInvalidateTimerHandle` (`self.TimerHandle`)))
  (if (`local.ExternalTimer`)
    (bind _returnvalue (`KismetSystemLibrary.K2_SetTimerDelegate` (`|CreateDelegate` :!event `ExternalUpdateTimer`) (`self.Substep`) true))
    (set `self.TimerHandle` _returnvalue)
    (else
      (bind _returnvalue_2 (`KismetSystemLibrary.K2_SetTimerDelegate` (`|CreateDelegate` :!event `UpdateTimer`) (`self.Substep`) true))
      (set `self.TimerHandle` _returnvalue_2))))

(fn `UpdateTimer`
  (if (select `bool` (`self.ReverseTimer`) :`false` (>= (`self.TimerAlpha`) 1.0) :`true` (<= (`self.TimerAlpha`) 0.0))
    (`KismetSystemLibrary.K2_ClearAndInvalidateTimerHandle` (`self.TimerHandle`))
    (if (`self.ReverseTimer`)
      (`self.CE_TimerFinishedDeactivate`)
      (else
        (`self.CE_TimerFinishedActivate`)))
    (else
      (set `self.TimerAlpha` (+ (* (* (/ 1.0 (`self.Duration`)) (`self.Substep`)) (`KismetMathLibrary.SelectFloat` -1.0 1.0 (`self.ReverseTimer`))) (`self.TimerAlpha`)))
      (`self.UpdateHandler` (`self.TimerAlpha`)))))