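; Actor component that bounces lasers off its owner by spawning a secondary SC_Emitter for each incoming laser.
; A map pairs each input laser with its emitter, which is added on hit start, repositioned on update and destroyed on stop.
; Force activation and deactivation replay those events over the owner AC_Handler's filtered lasers.
; MirrorLocationRotation supplies emitter transforms, but its only node, a normal-based reflection, is unconnected.
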(event `self.ReceiveBeginPlay`
  (bind _returnvalue (`Actor.GetComponentByClass` (`self.GetOwner`) "/Game/Blueprints/Refraction/AC_Handler.AC_Handler_C"))
  (`/Engine/EditorBlueprintResources/StandardMacros.IsValid` _returnvalue
    (:`Is Valid`
      (set `self.Owning Handler` _returnvalue))))

(event `/Game/Blueprints/Refraction/BPI_Lasers.LaserStartHitting`
  (params (Input :type "/Game/Blueprints/Refraction/A_Laser Object Reference") (`Hit Info` :type "HitResult Structure"))
  (`/Engine/EditorBlueprintResources/StandardMacros.IsValid` Input
    (:`Is Valid`
      (if (not (`BlueprintMapLibrary.Map_Contains` (`self.EmitterBounceMap`) Input))
        (`self.SpawnLaser` Input `Hit Info`)))))

(event `/Game/Blueprints/Refraction/BPI_Lasers.LaserStopHitting`
  (params (Input :type "/Game/Blueprints/Refraction/A_Laser Object Reference"))
  (`self.RemoveLaser` Input))

(event `/Game/Blueprints/Refraction/BPI_Lasers.LaserUpdateHitting`
  (params (Input :type "/Game/Blueprints/Refraction/A_Laser Object Reference") (`Hit Info` :type "HitResult Structure"))
  (bind (_location _rotation) (`self.MirrorLocationRotation` `Hit Info`))
  (bind (_value _returnvalue) (`BlueprintMapLibrary.Map_Find` (`self.EmitterBounceMap`) Input))
  (if _returnvalue
    (`SceneComponent.K2_SetWorldLocationAndRotation` _value _location _rotation false false)))

(event `/Game/Blueprints/Refraction/BPI_Lasers.ForceActivation`
  (params (ApplyConditions :type Boolean))
  (for _array_element (`/Game/Blueprints/Refraction/AC_Handler.FilteredLasers` (`self.Owning Handler`))
    (bind (_value _returnvalue) (`/Game/Blueprints/Refraction/A_Laser.GetHitByHandler` _array_element (`self.Owning Handler`)))
    (if _returnvalue
      (`self.LaserStartHitting` _array_element _value))))

(event `/Game/Blueprints/Refraction/BPI_Lasers.ForceDeactivation`
  (params (ApplyConditions :type Boolean))
  (for _array_element (`/Game/Blueprints/Refraction/AC_Handler.FilteredLasers` (`self.Owning Handler`))
    (`self.LaserStopHitting` _array_element)))

(fn `RemoveLaser`
  (params (InputPin :type "/Game/Blueprints/Refraction/A_Laser Object Reference"))
  (locals (`L-RemoveItem` :type "/Game/Blueprints/Refraction/SC_Emitter Object Reference"))
  (bind (_value _returnvalue) (`BlueprintMapLibrary.Map_Find` (`self.EmitterBounceMap`) (`local.InputPin`)))
  (if _returnvalue
    (bind _output_get (set `local.L-RemoveItem` _value))
    (`/Game/Blueprints/Refraction/SC_Emitter.LaserStopHitting` _output_get null)
    (`self.K2_DestroyComponent` (`local.L-RemoveItem`))
    (`BlueprintMapLibrary.Map_Remove` (`self.EmitterBounceMap`) (`local.InputPin`))))

(fn `SpawnLaser`
  (params (`Laser In` :type "/Game/Blueprints/Refraction/A_Laser Object Reference") (`Hit Info` :type "HitResult Structure"))
  (bind _returnvalue (`Actor.GetTransform` (`self.GetOwner`)))
  (bind (_location _rotation) (`self.MirrorLocationRotation` (`local.Hit Info`)))
  (bind _returnvalue_2 (`|AddComponentByClass` (`self.GetOwner`) "/Game/Blueprints/Refraction/SC_Emitter.SC_Emitter_C" false (`KismetMathLibrary.MakeTransform` (`KismetMathLibrary.InverseTransformLocation` _returnvalue _location) (`KismetMathLibrary.InverseTransformRotation` _returnvalue _rotation))))
  (`BlueprintMapLibrary.Map_Add` (`self.EmitterBounceMap`) (`local.Laser In`) _returnvalue_2)
  (`/Game/Blueprints/Refraction/SC_Emitter.Activate Laser` _returnvalue_2))